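; Traffic light Blueprint that cycles red, yellow, green, then back through yellow to red.
; Tick feeds latent Delays that pace the cycle, with a shorter hold while yellow is showing.
; Each step switches on the Light index to show one of the three light components and hide the others.
; A Flow direction flips at red and green, making the index ping-pong between the ends.
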(event EventTick
  (params (DeltaSeconds :type Float%20%28single-precision%29))
  ;[1 1 1] Toggle Light
  (if (Rendering|IsVisible (Variables|Default|GetLuz_Amarela))
    (Utilities|FlowControl|Delay 3.0)
    (else
      (Utilities|FlowControl|Delay 1e+01)))
  (switch int (Variables|Default|GetLight)
    (:0
      (Rendering|SetVisibility (Variables|Default|GetLuz_Vermelha) true false)
      (Rendering|SetVisibility (Variables|Default|GetLuz_Amarela) false false)
      (Rendering|SetVisibility (Variables|Default|GetLuz_Verde) false false)
      (Variables|Default|SetFlow 1))
    (:1
      (Rendering|SetVisibility (Variables|Default|GetLuz_Vermelha) false false)
      (Rendering|SetVisibility (Variables|Default|GetLuz_Amarela) true false)
      (Rendering|SetVisibility (Variables|Default|GetLuz_Verde) false false))
    (:2
      (Rendering|SetVisibility (Variables|Default|GetLuz_Vermelha) false false)
      (Rendering|SetVisibility (Variables|Default|GetLuz_Amarela) false false)
      (Rendering|SetVisibility (Variables|Default|GetLuz_Verde) true false)
      (Variables|Default|SetFlow -1)))
  (Variables|Default|SetLight (+ (Variables|Default|GetLight) (Variables|Default|GetFlow))))

(fn ConstructionScript)